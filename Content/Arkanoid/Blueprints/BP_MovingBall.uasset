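; BP_MovingBall is the Arkanoid ball, a physics-driven sphere that moves at constant speed along diagonals.
; On BeginPlay, FireStart launches it with a randomized impulse toward positive X and negative Y.
; Every Tick, ClampVelocity forces the velocity magnitude to Speed and snaps its heading to the nearest XY diagonal.
; The snap rotates the vector 45 degrees, rounds yaw to 90-degree steps, then rotates it back.
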(event Custom|FireStart
  (Physics|AddImpulse (Variables|Default|GetSphere) (Math|Vector|MakeVector (Math|Random|RandomFloatinRange 4e+02 6e+02) (Math|Random|RandomFloatinRange -4e+02 -6e+02) 0.0) "None" false))

(event Custom|ClampVelocity
  (bind _returnvalue (Math|Rotator|MakeRotator 0.0 0.0 45.0))
  (bind _returnvalue_2 (Transformation|GetVelocity))
  (bind _speed (Variables|Default|GetSpeed))
  (bind _returnvalue_3 (Math|Vector|ClampVectorSize _returnvalue_2 _speed _speed))
  (Physics|SetPhysicsLinearVelocity (Variables|Default|GetSphere) (* (Math|Vector|UnrotateVector (Math|Rotator|GetRotationXVector (Math|Rotator|MakeRotator 0.0 0.0 (|((round((A/B)))*B) (.yaw (Math|Rotator|MakeRotfromX (Math|Vector|RotateVector _returnvalue_3 _returnvalue))) 9e+01))) _returnvalue) (Math|Vector|VectorLength _returnvalue_3)) false "None"))

(event EventBeginPlay
  (CallFunction|FireStart))

(event EventTick
  (params (DeltaSeconds :type Float%20%28single-precision%29))
  (CallFunction|ClampVelocity))

(fn ConstructionScript)